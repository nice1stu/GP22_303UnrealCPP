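; Player controller for the Statue game that routes Enhanced Input to the possessed StatuePlayer pawn.
; On possession it caches the pawn, adds the IMC_Actions mapping context and puts a WBP_Counter widget on screen.
; Move input is forwarded to the pawn's Move function, while camera look applies yaw through the pawn and pitch on the controller itself.
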(event Input|EnhancedActionEvents|EnhancedInputActionIA_Move
  (params (ActionValue :type Vector%202D%20Structure) (ElapsedSeconds :type Float%20%28double-precision%29) (TriggeredSeconds :type Float%20%28double-precision%29) (InputAction :type Input%20Action%20Object%20Reference :default "/Game/Actions/IA_Move.IA_Move"))
  (:Triggered
    (Class|StatuePlayer|Move (Variables|Default|GetStatuePlayer) ActionValue)))

(event Input|EnhancedActionEvents|EnhancedInputActionIA_CameraLook
  (params (ActionValue :type Vector%202D%20Structure) (ElapsedSeconds :type Float%20%28double-precision%29) (TriggeredSeconds :type Float%20%28double-precision%29) (InputAction :type Input%20Action%20Object%20Reference :default "/Game/Actions/IA_CameraLook.IA_CameraLook"))
  (:Triggered
    (Pawn|Input|AddControllerYawInput (Variables|Default|GetStatuePlayer) (.x ActionValue))
    (Class|PlayerController|AddPitchInput (.y ActionValue))))

(event EventPossess
  (params (PossessedPawn :type Pawn%20Object%20Reference))
  (bind _asstatue_player (Utilities|Casting|CastToStatuePlayer PossessedPawn))
  (Variables|Default|SetStatuePlayer _asstatue_player)
  (Input|AddMappingContext (PlayerController|LocalPlayerSubsystems|GetEnhancedInputLocalPlayerSubsystem) "/Game/Actions/IMC_Actions.IMC_Actions" 0 "(bIgnoreAllPressedKeysUntilRelease=True,bForceImmediately=False)")
  (bind _returnvalue (UserInterface|CreateWidget "/Game/Statue/WBP_Counter.WBP_Counter_C" self))
  (UserInterface|Viewport|AddtoViewport _returnvalue 0))

(fn ConstructionScript)